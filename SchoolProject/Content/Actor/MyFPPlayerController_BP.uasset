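; MyFPPlayerController_BP is a player controller that toggles the pause menu when Tab is pressed.
; A FlipFlop alternates between creating a new PauseMenuMain_BP widget on screen with Game and UI input and a visible cursor, and removing it to restore game-only input with a hidden cursor.
; The game itself is never paused here, and BeginPlay and Tick do nothing.
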(event `Key|Tab`
  (params (Key :type "Key Structure"))
  (bind _returnvalue (`GameplayStatics.GetPlayerController` 0))
  (:`Pressed`
    (`/Engine/EditorBlueprintResources/StandardMacros.FlipFlop`
      (:`A`
        (bind _returnvalue_2 (`|CreateWidget` "/Game/UI/PauseMenu/PauseMenuMain_BP.PauseMenuMain_BP_C" _returnvalue))
        (bind _output_get (set `self.PauseMenu` _returnvalue_2))
        (`UserWidget.AddToViewport` _output_get 0)
        (`WidgetBlueprintLibrary.SetInputMode_GameAndUIEx` _returnvalue null)
        (set `self.bShowMouseCursor` true))
      (:`B`
        (`Widget.RemoveFromParent` (`self.PauseMenu`))
        (`WidgetBlueprintLibrary.SetInputMode_GameOnly` _returnvalue)
        (set `self.bShowMouseCursor` false)))))

(event `self.ReceiveBeginPlay`)

(fn `UserConstructionScript`)