(event `self.ReceiveBeginPlay`
  (set `self.Name"Date"` (`KismetStringLibrary.Conv_DoubleToString` (`GameplayStatics.GetRealTimeSeconds`)))
  (bind _returnvalue (`|CreateWidget` "/Game/Actor/HUD/UMG/GameHUD.GameHUD_C"))
  (bind _output_get (set `self.GameHUDWidget` _returnvalue))
  (`UserWidget.AddToViewport` _output_get 0))

(event `Key|I`
  (params (Key :type "Key Structure"))
  (bind _gamehudwidget (`self.GameHUDWidget`))
  (bind _gamehudwidget_2 (`self.GameHUDWidget`))
  (bind _inventorymenu (`/Game/Actor/HUD/UMG/GameHUD.InventoryMenu` _gamehudwidget))
  ;[1 1 1] Bring up inv menu
  (:`Pressed`
    (if (`/Game/Actor/HUD/UMG/GameHUD.InventoryActive` _gamehudwidget)
      (`/Engine/EditorBlueprintResources/StandardMacros.FlipFlop`
        (:`A`
          (`Widget.SetVisibility` _inventorymenu "Visible")
          (set `self.MenuOpen` true)
          (`self.EnableMouseCursor`)
          (`UserWidget.PlayAnimation` _gamehudwidget_2 (`/Game/Actor/HUD/UMG/GameHUD.InventoryFlyingIN` _gamehudwidget_2) 0.0 1 "Forward" 1.0))
        (:`B`
          (`UserWidget.PlayAnimation` _gamehudwidget (`/Game/Actor/HUD/UMG/GameHUD.InventoryFlyingOut` _gamehudwidget) 0.0 1 "Forward" 1.0)
          (set `self.MenuOpen` false)
          (`self.DisableMouseCursor`)
          (`KismetSystemLibrary.Delay` 0.75)
          (`Widget.SetVisibility` _inventorymenu "Hidden"))))))

(event `Key|E`
  (params (Key :type "Key Structure"))
  ;[1 1 1] Pickup items
  (:`Pressed`
    (if (< (`KismetArrayLibrary.Array_Length` (`/Game/Actor/HUD/UMG/GameHUD.Inventory_arr` (`self.GameHUDWidget`))) 15)
      (`self.PickupItem`)
      (else
        (`KismetSystemLibrary.PrintString` "Inventory Full")))))

(event `self.ReceiveTick`
  (params (DeltaSeconds :type "Float (single-precision)"))
  (if (<= (`self.HealthValue`) 0.0)
    (`KismetSystemLibrary.QuitGame` null "Quit")))

(event `/Game/Actor/HUD/ActionInteface.DropAction`
  (params (InActor :type "Actor Object Reference"))
  ;[1 1 1] Drop items
  (`self.SetActorHiddenInGame` InActor false)
  (`self.SetActorEnableCollision` InActor true)
  (`self.K2_SetActorTransform` InActor (`SceneComponent.K2_GetComponentToWorld` (`self.DropLocation`)) false false))

(event `Key|One`
  (params (Key :type "Key Structure"))
  (:`Pressed`
    (bind _returnvalue (`GameplayStatics.CreateSaveGameObject` "/Game/Saves/MySaveGame_BP.MySaveGame_BP_C"))
    (bind _output_get (set `self.Save Slot` _returnvalue))
    (bind _output_get_2 (set `self.PlayerLocation` (`self.K2_GetActorLocation`)))
    (set `/Game/Saves/MySaveGame_BP.Location` _output_get_2 _output_get)
    (bind _output_get_3 (set `/Game/Saves/MySaveGame_BP.Save Name` (`self.Name"Date"`) _output_get))
    (`GameplayStatics.SaveGameToSlot` (`self.Save Slot`) _output_get_3)
    (`KismetSystemLibrary.PrintString` "Game Saved")))

(event `Key|Two`
  (params (Key :type "Key Structure"))
  (bind _name_date_ (`self.Name"Date"`))
  (:`Pressed`
    (`GameplayStatics.CreateSaveGameObject` "/Game/Saves/MySaveGame_BP.MySaveGame_BP_C")
    (bind _returnvalue (`GameplayStatics.DoesSaveGameExist` _name_date_))
    (if _returnvalue
      (bind _returnvalue_2 (`GameplayStatics.LoadGameFromSlot` _name_date_))
      (bind _asmy_save_game_bp (cast `/Game/Saves/MySaveGame_BP` _returnvalue_2))
      (bind _output_get (set `self.PlayerLocation` (`/Game/Saves/MySaveGame_BP.Location` _asmy_save_game_bp)))
      (`self.K2_SetActorLocation` _output_get)
      (`KismetSystemLibrary.PrintString` "Save Loaded")
      (else
        (`KismetSystemLibrary.PrintString` "No save")))))

(event `InputAction|Jump`
  (params (Key :type "Key Structure"))
  (:`Pressed`
    (if (not (`NavMovementComponent.IsFalling` (`self.CharacterMovement`)))
      (`self.Jump`)
      (set `self.Energy` (- (`self.Energy`) 0.07)))))

(fn `DisableMouseCursor`
  (bind _returnvalue (`GameplayStatics.GetPlayerController` 0))
  (set `PlayerController.bShowMouseCursor` false _returnvalue)
  (bind _asmy_hud (cast `/Game/Actor/HUD/MyHUD` (`PlayerController.GetHUD` _returnvalue)))
  (set `/Game/Actor/HUD/MyHUD.ShowCrosshair` true _asmy_hud)
  (`WidgetBlueprintLibrary.SetInputMode_GameOnly` _returnvalue))

(fn `EnableMouseCursor`
  (bind _returnvalue (`GameplayStatics.GetPlayerController` 0))
  (set `PlayerController.bShowMouseCursor` true _returnvalue)
  (bind _asmy_hud (cast `/Game/Actor/HUD/MyHUD` (`PlayerController.GetHUD` _returnvalue)))
  (set `/Game/Actor/HUD/MyHUD.ShowCrosshair` false _asmy_hud)
  (`WidgetBlueprintLibrary.SetInputMode_GameAndUIEx` _returnvalue null))

(fn `UserConstructionScript`)