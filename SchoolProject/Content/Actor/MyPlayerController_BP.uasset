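; Player controller Blueprint that toggles the pause menu with the TAB input action.
; A FlipFlop alternates between creating and showing a new PauseMenuMain_BP widget with Game and UI input and a visible cursor, and removing it to restore game-only input.
; The game itself is never paused, and the HUD graph is empty.
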(event `InputAction|TAB`
  (params (Key :type "Key Structure"))
  (:`Pressed`
    (`/Engine/EditorBlueprintResources/StandardMacros.FlipFlop`
      (:`A`
        (bind _returnvalue (`|CreateWidget` "/Game/UI/PauseMenu/PauseMenuMain_BP.PauseMenuMain_BP_C"))
        (bind _output_get (set `self.PauseMenuVar` _returnvalue))
        (`UserWidget.AddToViewport` _output_get 0)
        (`WidgetBlueprintLibrary.SetInputMode_GameAndUIEx` self null "DoNotLock" false)
        (set `self.bShowMouseCursor` true))
      (:`B`
        (`Widget.RemoveFromParent` (`self.PauseMenuVar`))
        (`WidgetBlueprintLibrary.SetInputMode_GameOnly` self)
        (set `self.bShowMouseCursor` false)))))

(event `InputAction|Inventory`
  (params (Key :type "Key Structure")))

(fn `UserConstructionScript`)