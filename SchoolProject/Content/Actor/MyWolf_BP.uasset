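; MyWolf_BP is a wolf enemy actor that tracks attack and death state.
; An AttackingRange overlap sets IsAttacking when MyFPCharacter_BP enters and clears it when any overlap ends, without checking which actor left.
; Tick polls Health and, at zero or below, sets IsDead and destroys the actor after a delay.
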(event `self.ReceiveActorBeginOverlap`
  (params (OtherActor :type "Actor Object Reference")))

(event `self.ReceiveTick`
  (params (DeltaSeconds :type "Float (single-precision)"))
  (if (<= (`self.Health`) 0.0)
    (set `self.IsDead` true)
    (`KismetSystemLibrary.Delay` 20.0)
    (`self.K2_DestroyActor`)))

(event `self.AttackingRange.OnComponentBeginOverlap`
  (params (OverlappedComponent :type "PrimitiveComponent Object Reference") (OtherActor :type "Actor Object Reference") (OtherComp :type "PrimitiveComponent Object Reference") (OtherBodyIndex :type Integer) (bFromSweep :type Boolean) (SweepResult :type "HitResult Structure (by ref)"))
  (cast `/Game/Actor/MyFPCharacter_BP` OtherActor)
  (set `self.IsAttacking` true))

(event `self.AttackingRange.OnComponentEndOverlap`
  (params (OverlappedComponent :type "PrimitiveComponent Object Reference") (OtherActor :type "Actor Object Reference") (OtherComp :type "PrimitiveComponent Object Reference") (OtherBodyIndex :type Integer))
  (set `self.IsAttacking` false))

(fn `UserConstructionScript`)