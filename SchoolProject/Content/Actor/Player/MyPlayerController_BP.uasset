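; Player controller that handles menu toggling and HUD-to-character linking.
; P opens or closes a SettingsUI widget, whose CloseRequested event shares the same close path.
; TAB uses a FlipFlop to show or remove PauseMenuMain_BP, and both menus switch input mode and cursor without pausing the game here.
; FixUI points every top-level GameHUD widget at the controlled MyFPCharacter_BP.
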(event `FixUI`
  (bind _foundwidgets (`WidgetBlueprintLibrary.GetAllWidgetsOfClass` "/Game/Actor/HUD/UMG/GameHUD.GameHUD_C"))
  (for _array_element _foundwidgets
    (bind _asmy_fpcharacter_bp (cast `/Game/Actor/Player/MyFPCharacter_BP` (`self.K2_GetPawn`)))
    (set `/Game/Actor/HUD/UMG/GameHUD.MyCharacter` _asmy_fpcharacter_bp _array_element)))

(event `Key|P`
  (params (Key :type "Key Structure"))
  (:`Pressed`
    (if (`self.SettingsOpen`)
      (`Widget.RemoveFromParent` (stale _returnvalue) :!label _label)
      (`WidgetBlueprintLibrary.SetInputMode_GameOnly` self)
      (set `self.bShowMouseCursor` false)
      (set `self.SettingsOpen` false)
      (else
        (bind _returnvalue (`|CreateWidget` "/Game/UI/SettingsUI.SettingsUI_C"))
        (add `/Game/UI/SettingsUI.CloseRequested` _returnvalue (delegate `CloseRequested`))
        (`UserWidget.AddToViewport` _returnvalue 0)
        (`WidgetBlueprintLibrary.SetInputMode_GameAndUIEx` self _returnvalue)
        (set `self.bShowMouseCursor` true)
        (set `self.SettingsOpen` true)))))

(event `CloseRequested`
  (goto _label))

(event `InputAction|TAB`
  (params (Key :type "Key Structure"))
  (:`Pressed`
    (`/Engine/EditorBlueprintResources/StandardMacros.FlipFlop`
      (:`A`
        (bind _returnvalue (`|CreateWidget` "/Game/UI/PauseMenu/PauseMenuMain_BP.PauseMenuMain_BP_C"))
        (bind _output_get (set `self.PauseMenuVar` _returnvalue))
        (`UserWidget.AddToViewport` _output_get 0)
        (`WidgetBlueprintLibrary.SetInputMode_GameAndUIEx` self null "DoNotLock" false)
        (set `self.bShowMouseCursor` true))
      (:`B`
        (`Widget.RemoveFromParent` (`self.PauseMenuVar`))
        (`WidgetBlueprintLibrary.SetInputMode_GameOnly` self)
        (set `self.bShowMouseCursor` false)))))

(event `InputAction|Inventory`
  (params (Key :type "Key Structure")))

(fn `UserConstructionScript`)