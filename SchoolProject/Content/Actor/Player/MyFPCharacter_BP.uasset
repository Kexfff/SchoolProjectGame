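; First-person player character with an eight-slot weapon inventory, health regeneration, jump energy cost and HUD panels for inventory and skills.
; Inventory items are actors that spawn the selected weapon on the hand socket and become pickups when dropped.
; Firing works only while sighting, looping on the weapon's fire rate and saving rounds to the item; reloading draws from shared storage.
; Save/load logic exists but is never triggered.
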(event `self.ReceiveBeginPlay`
  ;[1 1 1] Viewport Setup
  (set `self.Name"Date"` (`KismetStringLibrary.Conv_DoubleToString` (`GameplayStatics.GetRealTimeSeconds`)))
  (bind _returnvalue (`|CreateWidget` "/Game/Actor/HUD/UMG/GameHUD.GameHUD_C"))
  (bind _output_get (set `self.GameHUDWidget` _returnvalue))
  (`UserWidget.AddToViewport` _output_get 0))

(event `self.ReceiveTick`
  (params (DeltaSeconds :type "Float (single-precision)"))
  (bind _healthvalue (`self.HealthValue`))
  (if (<= (`self.HealthValue`) 0.0)
    (`KismetSystemLibrary.QuitGame` null "Quit")
    (elif (< _healthvalue 1.0)
      (set `self.HealthValue` (+ _healthvalue (`self.RegenerationRate`))))))

(event `InputAction|Drop`
  (params (Key :type "Key Structure"))
  ;[1 1 1] Drop/ Change selected item
  (:`Pressed`
    (`self.DropItem` 0)
    (bind _output_get (set `self.SelectedItem` (`KismetMathLibrary.Clamp` (`KismetMathLibrary.Clamp` (`self.SelectedItem`) 0 (- (`KismetArrayLibrary.Array_Length` (`self.InventoryItems`)) 1)) 0 7)))
    (`self.HighlightSelected` _output_get)
    (`self.AddWeaponToViewport` _output_get)))

(event `InputAction|SelectItemNext`
  (params (Key :type "Key Structure"))
  ;[1 1 1] Drop/ Change selected item
  (:`Pressed`
    (bind _output_get (set `self.SelectedItem` (`KismetMathLibrary.Clamp` (`KismetMathLibrary.Clamp` (+ (`self.SelectedItem`) 1) 0 (- (`KismetArrayLibrary.Array_Length` (`self.InventoryItems`)) 1)) 0 7)))
    (`self.HighlightSelected` _output_get)
    (`self.AddWeaponToViewport` _output_get)))

(event `InputAction|SelectItemPrev`
  (params (Key :type "Key Structure"))
  ;[1 1 1] Drop/ Change selected item
  (:`Pressed`
    (bind _output_get (set `self.SelectedItem` (`KismetMathLibrary.Clamp` (`KismetMathLibrary.Clamp` (+ (`self.SelectedItem`) -1) 0 (- (`KismetArrayLibrary.Array_Length` (`self.InventoryItems`)) 1)) 0 7)))
    (`self.HighlightSelected` _output_get)
    (`self.AddWeaponToViewport` _output_get)))

(event `Key|NumPadTwo`
  (params (Key :type "Key Structure"))
  (:`Pressed`
    (set `self.HealthValue` (- (`self.HealthValue`) 0.2))))

(event `InputAction|Reloading`
  (params (Key :type "Key Structure"))
  (bind _roundsstorage (`self.RoundsStorage`))
  ;[1 1 1] Reloading
  (:`Pressed`
    (for (_array_element _array_index) (`self.InventoryItems`)
      (if (== _array_index (`self.SelectedItem`))
        (bind _asinv_weapon_parent (cast `/Game/Blueprints/Inventory/InventoryActors/Inv_WeaponParent` _array_element))
        (bind _asweapon_actor_parent (cast `/Game/Blueprints/Inventory/Weapons/WeaponActorParent` (`self.LastAttachedActor`))
          (:`then`
            (bind _rounds (`/Game/Blueprints/Inventory/InventoryActors/Inv_WeaponParent.Rounds` _asinv_weapon_parent))
            (bind _returnvalue (`KismetMathLibrary.Clamp` (- (`.Rounds_6_100049EB429FD3BAD12F87ACE865E350` (break `/Game/Blueprints/Inventory/WeaponStruct` (`/Game/Blueprints/Inventory/Weapons/WeaponActorParent.WeaponStruct` _asweapon_actor_parent))) _rounds) 0 _roundsstorage))
            (bind _output_get (set `self.TempRounds` _returnvalue))
            (set `/Game/Blueprints/Inventory/InventoryActors/Inv_WeaponParent.Rounds` (+ _returnvalue _rounds) _asinv_weapon_parent)
            (set `self.RoundsStorage` (- _roundsstorage _output_get)))
          (:`CastFailed`
            (set `/Game/Blueprints/Inventory/InventoryActors/Inv_WeaponParent.Rounds` 10 _asinv_weapon_parent)))))))

(event `InputAction|Jump`
  (params (Key :type "Key Structure"))
  ;[1 1 1] Jumping
  (:`Pressed`
    (if (not (`NavMovementComponent.IsFalling` (`self.CharacterMovement`)))
      (`self.Jump`)
      (set `self.Energy` (- (`self.Energy`) 0.07)))))

(event `Key|RightMouseButton`
  (params (Key :type "Key Structure"))
  (bind _fpcameracomponent (`self.FPCameraComponent`))
  (bind _sight (`self.Sight`))
  (:`Pressed`
    (if (`self.IsWeaponEquiped`)
      (bind _asweapon_actor_parent (cast `/Game/Blueprints/Inventory/Weapons/WeaponActorParent` (`self.LastAttachedActor`)))
      (`SceneComponent.K2_SetRelativeTransform` _sight (`SceneComponent.GetSocketTransform` (`self.Weapon`) (`/Game/Blueprints/Inventory/Weapons/WeaponActorParent.SocketName` _asweapon_actor_parent) "RTS_Component") false false)
      (set `self.IsSighting` true)
      (`self.SetMaxSpeed` 100.0)
      (`KismetSystemLibrary.Delay` 0.2)
      (`ActorComponent.Deactivate` _fpcameracomponent)
      (`ActorComponent.Activate` (`self.Sight`) false)))
  (:`Released`
    (`ActorComponent.Deactivate` _sight)
    (`ActorComponent.Activate` _fpcameracomponent false)
    (`self.SetMaxSpeed` (`self.DefaultMaxSpeed`))
    (set `self.IsSighting` false)))

(event `InputAction|Inventory`
  (params (Key :type "Key Structure"))
  ;[1 1 1] Open/Close inventory
  (:`Pressed`
    (`/Game/Actor/HUD/UMG/GameHUD.RefreshInventory` (`self.GameHUDWidget`))
    (if (`self.IsInventoryOpened`)
      (`self.CloseInventory`)
      (else
        (if (`self.IsSkillOpened`)
          (`self.CloseSkills`))
        (`self.OpenInventory`)))))

(event `InputAction|Skills`
  (params (Key :type "Key Structure"))
  ;[1 1 1] Open/Close inventory
  (:`Pressed`
    (if (`self.IsSkillOpened`)
      (`self.CloseSkills`)
      (else
        (if (`self.IsInventoryOpened`)
          (`self.CloseInventory`))
        (`self.OpenSkills`)))))

(event `Key|One`
  (params (Key :type "Key Structure"))
  (bind _gamehudwidget (`self.GameHUDWidget`))
  (:`Pressed`
    (if (`/Game/Actor/HUD/UMG/GameHUD.IsActionMenuActivated` _gamehudwidget)
      (`self.MoveItem` 0 (`/Game/Actor/HUD/UMG/GameHUD.InventorySlot` _gamehudwidget)))))

(event `Key|Two`
  (params (Key :type "Key Structure"))
  (bind _gamehudwidget (`self.GameHUDWidget`))
  (:`Pressed`
    (if (`/Game/Actor/HUD/UMG/GameHUD.IsActionMenuActivated` _gamehudwidget)
      (`self.MoveItem` 1 (`/Game/Actor/HUD/UMG/GameHUD.InventorySlot` _gamehudwidget)))))

(event `Key|Three`
  (params (Key :type "Key Structure"))
  (bind _gamehudwidget (`self.GameHUDWidget`))
  (:`Pressed`
    (if (`/Game/Actor/HUD/UMG/GameHUD.IsActionMenuActivated` _gamehudwidget)
      (`self.MoveItem` 2 (`/Game/Actor/HUD/UMG/GameHUD.InventorySlot` _gamehudwidget)))))

(event `Key|Four`
  (params (Key :type "Key Structure"))
  (bind _gamehudwidget (`self.GameHUDWidget`))
  (:`Pressed`
    (if (`/Game/Actor/HUD/UMG/GameHUD.IsActionMenuActivated` _gamehudwidget)
      (`self.MoveItem` 3 (`/Game/Actor/HUD/UMG/GameHUD.InventorySlot` _gamehudwidget)))))

(event `Key|Five`
  (params (Key :type "Key Structure"))
  (bind _gamehudwidget (`self.GameHUDWidget`))
  (:`Pressed`
    (if (`/Game/Actor/HUD/UMG/GameHUD.IsActionMenuActivated` _gamehudwidget)
      (`self.MoveItem` 4 (`/Game/Actor/HUD/UMG/GameHUD.InventorySlot` _gamehudwidget)))))

(event `Key|Six`
  (params (Key :type "Key Structure"))
  (bind _gamehudwidget (`self.GameHUDWidget`))
  (:`Pressed`
    (if (`/Game/Actor/HUD/UMG/GameHUD.IsActionMenuActivated` _gamehudwidget)
      (`self.MoveItem` 5 (`/Game/Actor/HUD/UMG/GameHUD.InventorySlot` _gamehudwidget)))))

(event `Key|Seven`
  (params (Key :type "Key Structure"))
  (bind _gamehudwidget (`self.GameHUDWidget`))
  (:`Pressed`
    (if (`/Game/Actor/HUD/UMG/GameHUD.IsActionMenuActivated` _gamehudwidget)
      (`self.MoveItem` 6 (`/Game/Actor/HUD/UMG/GameHUD.InventorySlot` _gamehudwidget)))))

(event `Key|Eight`
  (params (Key :type "Key Structure"))
  (bind _gamehudwidget (`self.GameHUDWidget`))
  (:`Pressed`
    (if (`/Game/Actor/HUD/UMG/GameHUD.IsActionMenuActivated` _gamehudwidget)
      (`self.MoveItem` 7 (`/Game/Actor/HUD/UMG/GameHUD.InventorySlot` _gamehudwidget)))))

(event `Key|Add`
  (params (Key :type "Key Structure"))
  ;[1 1 1] Debug Skills TODO delete
  (:`Pressed`
    (set `self.SkillsPoints` (+ (`self.SkillsPoints`) 1))))

(event `Key|NumPadOne`
  (params (Key :type "Key Structure"))
  ;[1 1 1] Debug Skills TODO delete
  (:`Pressed`
    (for _array_element (`self.SkillsArray`)
      (`KismetSystemLibrary.PrintString` (`KismetStringLibrary.Conv_DoubleToString` _array_element)))))

(event `InputAction|Fire`
  (params (Key :type "Key Structure"))
  (bind _firing (`self.Firing`))
  (:`Pressed`
    (set `self.IsFiring` true)
    (if (`self.IsFiring`) :!label _label
      (if (`self.IsWeaponEquiped`)
        (if (`self.IsSighting`)
          (bind _asweapon_actor_parent (cast `/Game/Blueprints/Inventory/Weapons/WeaponActorParent` (`self.LastAttachedActor`)))
          (bind _asinv_weapon_parent (cast `/Game/Blueprints/Inventory/InventoryActors/Inv_WeaponParent` (`|GetArrayItem` (`self.InventoryItems`) (`self.SelectedItem`))))
          (bind _rounds (`/Game/Blueprints/Inventory/InventoryActors/Inv_WeaponParent.Rounds` _asinv_weapon_parent))
          (bind _output_get (set `self.RoundsLeft` _rounds))
          (if (> _rounds 0)
            (`FiringComponent.SetReference` _firing (`self.WeaponMesh_CPP`))
            (`FiringComponent.Fire` _firing)
            (`self.AddControllerPitchInput` -1.0)
            (set `self.RoundsLeft` (- _output_get 1))
            (bind (_isautomatic _firerate _rounds_2 _sound) (break `/Game/Blueprints/Inventory/WeaponStruct` (`/Game/Blueprints/Inventory/Weapons/WeaponActorParent.WeaponStruct` _asweapon_actor_parent)))
            (`GameplayStatics.PlaySoundAtLocation` _sound (`self.PlayerLocation`) (struct) 1.0 1.0 0.0 null null null)
            (`KismetSystemLibrary.Delay` _firerate)
            (`self.SetCurrentRoundsLeft`)
            (goto _label))))))
  (:`Released`
    (set `self.IsFiring` false)))

(fn `AddItem`
  (params (InventoryClass :type "Actor Class Reference") (Mesh :type "StaticMesh Object Reference") (Scale :type "Float (double-precision)") (Rounds :type Integer))
  (bind _returnvalue (`|SpawnActorFromClass` InventoryClass (`KismetMathLibrary.MakeTransform` (0.0 0.0 0.0)) "Undefined" "OverrideRootScale" null null))
  (bind _asbp_inventory_actor (cast `/Game/Blueprints/Inventory/InventoryActors/BP_InventoryActor` _returnvalue))
  (set `/Game/Blueprints/Inventory/InventoryActors/BP_InventoryActor.ActorMesh` Mesh _asbp_inventory_actor)
  (set `/Game/Blueprints/Inventory/InventoryActors/BP_InventoryActor.Actor Scale` Scale _asbp_inventory_actor)
  (`KismetArrayLibrary.Array_Add` (`self.InventoryItems`) _asbp_inventory_actor)
  (`/Game/Actor/HUD/UMG/GameHUD.RefreshInventory` (`self.GameHUDWidget`))
  (`KismetSystemLibrary.PrintString` (`KismetStringLibrary.Conv_IntToString` Rounds))
  (bind _asinv_weapon_parent (cast `/Game/Blueprints/Inventory/InventoryActors/Inv_WeaponParent` _asbp_inventory_actor))
  (set `/Game/Blueprints/Inventory/InventoryActors/Inv_WeaponParent.Rounds` Rounds _asinv_weapon_parent)
  (`self.AddWeaponToViewport` (`self.SelectedItem`)))

(fn `AddRounds`
  (params (Amount :type Integer))
  (bind _roundsstorage (`self.RoundsStorage`))
  (bind _maxrounds (`self.MaxRounds`))
  (if (<= _roundsstorage _maxrounds)
    (set `self.RoundsStorage` (`KismetMathLibrary.Clamp` (+ _roundsstorage Amount) 0 _maxrounds))))

(fn `AddWeaponToViewport`
  (params (Integer :type Integer))
  (bind _gamehudwidget (`self.GameHUDWidget`))
  (bind _gamehudwidget_2 (`self.GameHUDWidget`))
  (bind _lastattachedactor (`self.LastAttachedActor`))
  (if (`KismetSystemLibrary.IsValid` _lastattachedactor) :!label _label
    (`self.K2_DestroyActor` _lastattachedactor)
    (set `self.IsWeaponEquiped` false)
    (set `self.LastAttachedActor` null)
    (`UserWidget.PlayAnimation` _gamehudwidget_2 (`/Game/Actor/HUD/UMG/GameHUD.RoundsOUT` _gamehudwidget_2) 0.0 1 "Forward" 1.0)
    (goto _label)
    (else
      (bind _asinv_weapon_parent (cast `/Game/Blueprints/Inventory/InventoryActors/Inv_WeaponParent` (`|GetArrayItem` (`self.InventoryItems`) Integer)))
      (bind _returnvalue (`|SpawnActorFromClass` (`/Game/Blueprints/Inventory/InventoryActors/Inv_WeaponParent.WeaponRef` _asinv_weapon_parent) (`KismetMathLibrary.MakeTransform` (0.0 0.0 0.0)) "Undefined" "OverrideRootScale" null null))
      (set `self.LastAttachedActor` _returnvalue)
      (bind _returnvalue_2 (`SceneComponent.K2_AttachToComponent` (`Actor.RootComponent` _returnvalue) (`self.Mesh`) "R_Weapon" "KeepRelative" "KeepRelative" "KeepRelative" true))
      (set `self.IsWeaponEquiped` _returnvalue_2)
      (`UserWidget.PlayAnimation` _gamehudwidget (`/Game/Actor/HUD/UMG/GameHUD.RoundsIN` _gamehudwidget) 0.0 1 "Forward" 1.0))))

(fn `CheckSkills`)

(fn `CloseInventory`
  (bind _gamehudwidget (`self.GameHUDWidget`))
  (`/Game/Actor/HUD/UMG/GameHUD.CloseActionMenu` _gamehudwidget)
  (`UserWidget.PlayAnimation` _gamehudwidget (`/Game/Actor/HUD/UMG/GameHUD.CloseInventory` _gamehudwidget) 0.0 1 "Forward" 1.0)
  (`self.DisableMouseCursor`)
  (`Widget.SetVisibility` (`/Game/Actor/HUD/UMG/GameHUD.Highlighter` _gamehudwidget) "Visible")
  (set `self.IsInventoryOpened` false))

(fn `CloseSkills`
  (bind _gamehudwidget (`self.GameHUDWidget`))
  (`UserWidget.PlayAnimation` _gamehudwidget (`/Game/Actor/HUD/UMG/GameHUD.SkillsOUT` _gamehudwidget) 0.0 1 "Forward" 1.0)
  (`self.DisableMouseCursor`)
  (set `self.IsSkillOpened` false))

(fn `DisableMouseCursor`
  (bind _returnvalue (`GameplayStatics.GetPlayerController` 0))
  (set `PlayerController.bShowMouseCursor` false _returnvalue)
  (bind _asmy_hud (cast `/Game/Actor/HUD/MyHUD` (`PlayerController.GetHUD` _returnvalue)))
  (set `/Game/Actor/HUD/MyHUD.ShowCrosshair` true _asmy_hud)
  (`WidgetBlueprintLibrary.SetInputMode_GameOnly` _returnvalue))

(fn `DropItem`
  (params (SlotNumber :type Integer))
  (bind _inventoryitems (`self.InventoryItems`))
  (bind _inventoryitems_2 (`self.InventoryItems`))
  (bind _output (`|GetArrayItem` _inventoryitems SlotNumber))
  (bind _output_2 (`|GetArrayItem` _inventoryitems_2 SlotNumber))
  (bind _pickupclass (`/Game/Blueprints/Inventory/InventoryActors/BP_InventoryActor.PickupClass` _output))
  (bind _actor_scale (`/Game/Blueprints/Inventory/InventoryActors/BP_InventoryActor.Actor Scale` _output_2))
  (if (> (`KismetArrayLibrary.Array_Length` _inventoryitems) 0)
    (bind _returnvalue (`|SpawnActorFromClass` _pickupclass (`KismetMathLibrary.Conv_VectorToTransform` (+ (+ (`self.K2_GetActorLocation`) (`self.BaseEyeHeight`)) (`KismetMathLibrary.GreaterGreater_VectorRotator` (100.0 0.0 0.0) (`self.GetControlRotation`)))) "Undefined" "OverrideRootScale" null null))
    (bind _asbasic_example (cast `/Game/Blueprints/Inventory/InventoryWorld/BasicExample` _returnvalue))
    (`KismetSystemLibrary.PrintString` (`KismetSystemLibrary.GetClassDisplayName` _pickupclass))
    (set `/Game/Blueprints/Inventory/InventoryWorld/BasicExample.InventoryClass` (`GameplayStatics.GetObjectClass` _output) _asbasic_example)
    (`StaticMeshComponent.SetStaticMesh` (`/Game/Blueprints/Inventory/InventoryWorld/BasicExample.StaticMesh` _asbasic_example) (`/Game/Blueprints/Inventory/InventoryActors/BP_InventoryActor.ActorMesh` _output))
    (set `/Game/Blueprints/Inventory/InventoryWorld/BasicExample.Scale` _actor_scale _asbasic_example)
    (bind _asinv_weapon_parent (cast `/Game/Blueprints/Inventory/InventoryActors/Inv_WeaponParent` _output_2))
    (bind _output_get (set `/Game/Blueprints/Inventory/InventoryWorld/BasicExample.Rounds` (`/Game/Blueprints/Inventory/InventoryActors/Inv_WeaponParent.Rounds` _asinv_weapon_parent) _asbasic_example))
    (`/Game/Blueprints/Inventory/InventoryWorld/BasicExample.OnSpawned` _asbasic_example _actor_scale _output_get)
    (`self.K2_DestroyActor` _output_2)
    (`KismetArrayLibrary.Array_Remove` _inventoryitems_2 SlotNumber)
    (`/Game/Actor/HUD/UMG/GameHUD.RefreshInventory` (`self.GameHUDWidget`))
    (`self.AddWeaponToViewport` (`self.SelectedItem`))))

(fn `EnableMouseCursor`
  (bind _returnvalue (`GameplayStatics.GetPlayerController` 0))
  (set `PlayerController.bShowMouseCursor` true _returnvalue)
  (bind _asmy_hud (cast `/Game/Actor/HUD/MyHUD` (`PlayerController.GetHUD` _returnvalue)))
  (set `/Game/Actor/HUD/MyHUD.ShowCrosshair` false _asmy_hud)
  (`WidgetBlueprintLibrary.SetInputMode_GameAndUIEx` _returnvalue null))

(fn `HighlightSelected`
  (params (Slot :type Integer))
  (bind _gamehudwidget (`self.GameHUDWidget`))
  (`|ExecutionSequence`
    (:`then_0`
      (if (== Slot 0)
        (`UserWidget.PlayAnimation` _gamehudwidget (`/Game/Actor/HUD/UMG/GameHUD.Choice0` _gamehudwidget) 0.0 1 "Forward" 1.0)))
    (:`then_1`
      (if (== Slot 1)
        (`UserWidget.PlayAnimation` _gamehudwidget (`/Game/Actor/HUD/UMG/GameHUD.Choice1` _gamehudwidget) 0.0 1 "Forward" 1.0)))
    (:`then_2`
      (if (== Slot 2)
        (`UserWidget.PlayAnimation` _gamehudwidget (`/Game/Actor/HUD/UMG/GameHUD.Choice2` _gamehudwidget) 0.0 1 "Forward" 1.0)))
    (:`then_3`
      (if (== Slot 3)
        (`UserWidget.PlayAnimation` _gamehudwidget (`/Game/Actor/HUD/UMG/GameHUD.Choice3` _gamehudwidget) 0.0 1 "Forward" 1.0)))
    (:`then_4`
      (if (== Slot 4)
        (`UserWidget.PlayAnimation` _gamehudwidget (`/Game/Actor/HUD/UMG/GameHUD.Choice4` _gamehudwidget) 0.0 1 "Forward" 1.0)))
    (:`then_5`
      (if (== Slot 5)
        (`UserWidget.PlayAnimation` _gamehudwidget (`/Game/Actor/HUD/UMG/GameHUD.Choice5` _gamehudwidget) 0.0 1 "Forward" 1.0)))
    (:`then_6`
      (if (== Slot 6)
        (`UserWidget.PlayAnimation` _gamehudwidget (`/Game/Actor/HUD/UMG/GameHUD.Choice6` _gamehudwidget) 0.0 1 "Forward" 1.0)))
    (:`then_7`
      (if (== Slot 7)
        (`UserWidget.PlayAnimation` _gamehudwidget (`/Game/Actor/HUD/UMG/GameHUD.Choice7` _gamehudwidget) 0.0 1 "Forward" 1.0)))))

(fn `MoveItem`
  (params (ToSlot :type Integer) (FromSlot :type Integer))
  (locals (FromSlotVar :type "/Game/Blueprints/Inventory/InventoryActors/BP_InventoryActor Object Reference") (ToSlotVar :type "/Game/Blueprints/Inventory/InventoryActors/BP_InventoryActor Object Reference"))
  (bind _inventoryitems (`self.InventoryItems`))
  (bind _output_get (set `local.FromSlotVar` (`|GetArrayItem` _inventoryitems FromSlot)))
  (bind _output_get_2 (set `local.ToSlotVar` (`|GetArrayItem` _inventoryitems ToSlot)))
  (`KismetArrayLibrary.Array_RemoveItem` _inventoryitems _output_get_2)
  (`KismetArrayLibrary.Array_RemoveItem` _inventoryitems _output_get)
  (`KismetArrayLibrary.Array_Insert` _inventoryitems (`local.FromSlotVar`) ToSlot)
  (`KismetArrayLibrary.Array_Insert` _inventoryitems (`local.ToSlotVar`) FromSlot))

(fn `OpenInventory`
  (bind _gamehudwidget (`self.GameHUDWidget`))
  (`UserWidget.PlayAnimation` _gamehudwidget (`/Game/Actor/HUD/UMG/GameHUD.OpenInventory` _gamehudwidget) 0.0 1 "Forward" 1.0)
  (`self.EnableMouseCursor`)
  (`Widget.SetVisibility` (`/Game/Actor/HUD/UMG/GameHUD.Highlighter` _gamehudwidget) "Hidden")
  (set `self.IsInventoryOpened` true)
  (return))

(fn `OpenSkills`
  (bind _gamehudwidget (`self.GameHUDWidget`))
  (`UserWidget.PlayAnimation` _gamehudwidget (`/Game/Actor/HUD/UMG/GameHUD.SkillsIN` _gamehudwidget) 0.0 1 "Forward" 1.0)
  (`self.EnableMouseCursor`)
  (set `self.IsSkillOpened` true)
  (return))

(fn `SetCurrentRoundsLeft`
  (for (_array_element _array_index) (`self.InventoryItems`)
    (if (== _array_index (`self.SelectedItem`))
      (bind _asinv_weapon_parent (cast `/Game/Blueprints/Inventory/InventoryActors/Inv_WeaponParent` _array_element))
      (set `/Game/Blueprints/Inventory/InventoryActors/Inv_WeaponParent.Rounds` (`self.RoundsLeft`) _asinv_weapon_parent))))

(fn `SetSelectedItemIndex`
  (params (NewIndex :type Integer))
  (set `self.SelectedItem` (`KismetMathLibrary.Clamp` NewIndex 0 (- (`KismetArrayLibrary.Array_Length` (`self.InventoryItems`)) 1))))

(fn `TakeDamage`
  (params (Damage :type "Float (double-precision)"))
  (set `self.HealthValue` (- (`self.HealthValue`) Damage)))

(fn `UseItem`
  (params (Slot :type Integer))
  (bind _inventoryitems (`self.InventoryItems`))
  (`KismetSystemLibrary.PrintString` "Item was used")
  (if (> (`KismetArrayLibrary.Array_Length` (`self.InventoryItems`)) 0)
    (`self.K2_DestroyActor` (`|GetArrayItem` _inventoryitems Slot))
    (`KismetArrayLibrary.Array_Remove` _inventoryitems Slot)
    (`/Game/Actor/HUD/UMG/GameHUD.RefreshInventory` (`self.GameHUDWidget`))))

(fn `UserConstructionScript`
  (set `self.DefaultMaxSpeed` (`CharacterMovementComponent.MaxCustomMovementSpeed` (`self.CharacterMovement`))))