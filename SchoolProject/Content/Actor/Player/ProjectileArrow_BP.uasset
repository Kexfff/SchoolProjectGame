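; Player arrow projectile that stays inactive until launched, damages characters and wolves it overlaps, and turns into an item on impact.
; StartTimer arms it and starts a self-destruct delay, with the firing owner then excluded from damage and hits.
; Each tick, complex then simple sphere traces look ahead, either stopping it to spawn a non-simulating item in its place or pitching it along its velocity.
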(event `StartTimer`
  (set `self.Fired` true)
  (`KismetSystemLibrary.Delay` 10.0)
  (`self.K2_DestroyActor`))

(event `self.ReceiveActorBeginOverlap`
  (params (OtherActor :type "Actor Object Reference"))
  (bind _asmy_fpcharacter_bp (cast `/Game/Actor/Player/MyFPCharacter_BP` OtherActor)
    (:`then`
      (if (not (and (== _asmy_fpcharacter_bp (`self.GetOwner`)) (`self.Fired`)))
        (`/Game/Actor/Player/MyFPCharacter_BP.DoDamage` _asmy_fpcharacter_bp (`self.damage`))))
    (:`CastFailed`
      ;[1 1 1] DO on Server
      (bind _asmy_wolf_bp (cast `/Game/Actor/MyWolf_BP` OtherActor))
      (set `/Game/Actor/MyWolf_BP.Health` (- (`/Game/Actor/MyWolf_BP.Health` _asmy_wolf_bp) (`self.damage`)) _asmy_wolf_bp))))

(event `self.ReceiveTick`
  (params (DeltaSeconds :type "Float (single-precision)"))
  (bind _sphere (`self.Sphere`))
  (bind _sphere_2 (`self.Sphere`))
  (bind _returnvalue (`SceneComponent.K2_GetComponentLocation` _sphere))
  (bind _returnvalue_2 (`SceneComponent.K2_GetComponentLocation` _sphere_2))
  (if (`self.Fired`)
    (bind (_outhit _returnvalue_3) (`KismetSystemLibrary.SphereTraceSingleByProfile` _returnvalue (+ (`SceneComponent.GetForwardVector` _sphere) _returnvalue) 5.0 "Arrow" true))
    (bind _isnotowner (`self.CheckForOwner` _outhit))
    (if (and _returnvalue_3 _isnotowner)
      (`self.TrySpawn` :!label _label)
      (else
        (bind (_outhit_2 _returnvalue_4) (`KismetSystemLibrary.SphereTraceSingleByProfile` _returnvalue_2 (+ (`SceneComponent.GetForwardVector` _sphere_2) _returnvalue_2) 5.0 "Arrow"))
        (bind _isnotowner_2 (`self.CheckForOwner` _outhit_2))
        (if (and _isnotowner_2 _returnvalue_4)
          (goto _label)
          (else
            (`self.AngleArrow`)))))))

(event `TrySpawn`
  (`MovementComponent.StopMovementImmediately` (`self.ProjectileMovement`))
  (`/Engine/EditorBlueprintResources/StandardMacros.DoOnce` false
    (:`Completed`
      (bind _returnvalue (`|SpawnActorFromClass` "/Game/ThirdPersonBP/InventoryImport/Items/Item.Item_C" (`KismetMathLibrary.MakeTransform` (.location (`self.GetTransform`)) (`KismetMathLibrary.MakeRotator` (.roll (.rotation (`self.GetTransform`))) (- (.pitch (.rotation (`self.GetTransform`))) -90.0) (.yaw (.rotation (`self.GetTransform`)))) (.scale (`self.GetTransform`))) "Undefined" "OverrideRootScale" null null))
      (`PrimitiveComponent.SetSimulatePhysics` (`/Game/ThirdPersonBP/InventoryImport/Items/Item.ItemMesh` _returnvalue) false)
      (set `/Game/ThirdPersonBP/InventoryImport/Items/Item.ItemID` 10 _returnvalue)
      (`/Game/ThirdPersonBP/InventoryImport/Items/Item.Update` _returnvalue)
      (`self.K2_DestroyActor`))))

(event `LaunchProjectileServer`
  (params (Speed :type "Float (double-precision)"))
  (`self.LaunchProjectile` Speed))

(event `AngleArrow`
  (`self.K2_SetActorRotation` (`KismetMathLibrary.MakeRotator` (.roll (`self.K2_GetActorRotation`)) (.pitch (`KismetMathLibrary.MakeRotFromX` (`self.GetVelocity`))) (.yaw (`self.K2_GetActorRotation`)))))

(fn `CheckForOwner`
  (params (Hit :type "HitResult Structure"))
  (returns (IsNotOwner :type Boolean))
  (bind (_bblockinghit _binitialoverlap _time _distance _location _impactpoint _normal _impactnormal _physmat _hitactor) (`GameplayStatics.BreakHitResult` Hit))
  (bind _returnvalue (`self.GetOwner`))
  (if (== _hitactor _returnvalue)
    (return false)
    (else
      (bind _asmy_fpcharacter_bp (cast `/Game/Actor/Player/MyFPCharacter_BP` _returnvalue)
        (:`then`
          (if (== _asmy_fpcharacter_bp _hitactor)
            (return false)
            (else
              (return true))))
        (:`CastFailed`
          (return true))))))

(fn `LaunchProjectile`
  (params (NewParam :type "Float (double-precision)"))
  (bind _projectilemovement (`self.ProjectileMovement`))
  (`ProjectileMovementComponent.SetVelocityInLocalSpace` _projectilemovement (* (`KismetMathLibrary.GetForwardVector` (struct)) NewParam))
  (`ActorComponent.Activate` _projectilemovement false))

(fn `UserConstructionScript`
  (`ActorComponent.SetAutoActivate` (`self.ProjectileMovement`) false))