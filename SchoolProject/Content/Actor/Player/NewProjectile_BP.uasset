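; Projectile actor that damages the first-person player character or a wolf on overlap, then destroys itself.
; Its movement component stays inactive until LaunchProjectile sets a local forward velocity at the given speed and activates it.
; Overlap subtracts Damage directly from the target's health variable through class casts, ignoring other actors.
; A short timer from BeginPlay destroys any projectile that hits neither target.
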(event `self.ReceiveBeginPlay`
  (`KismetSystemLibrary.Delay` 3.0)
  (`self.K2_DestroyActor` :!label _label))

(event `self.ReceiveActorBeginOverlap`
  (params (OtherActor :type "Actor Object Reference"))
  (bind _asmy_fpcharacter_bp (cast `/Game/Actor/Player/MyFPCharacter_BP` OtherActor)
    (:`then`
      (set `/Game/Actor/Player/MyFPCharacter_BP.HealthValue` (- (`/Game/Actor/Player/MyFPCharacter_BP.HealthValue` _asmy_fpcharacter_bp) (`self.damage`)) _asmy_fpcharacter_bp)
      (goto _label))
    (:`CastFailed`
      (bind _asmy_wolf_bp (cast `/Game/Actor/MyWolf_BP` OtherActor))
      (set `/Game/Actor/MyWolf_BP.Health` (- (`/Game/Actor/MyWolf_BP.Health` _asmy_wolf_bp) (`self.damage`)) _asmy_wolf_bp)
      (goto _label))))

(event `self.ReceiveTick`
  (params (DeltaSeconds :type "Float (single-precision)")))

(fn `LaunchProjectile`
  (params (NewParam :type "Float (double-precision)"))
  (bind _projectilemovement (`self.ProjectileMovement`))
  (`ProjectileMovementComponent.SetVelocityInLocalSpace` _projectilemovement (* (`KismetMathLibrary.GetForwardVector` (struct)) NewParam))
  (`ActorComponent.Activate` _projectilemovement false))

(fn `UserConstructionScript`
  (`ActorComponent.SetAutoActivate` (`self.ProjectileMovement`) false))