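; Buildable door Blueprint for the building system that swings open or closed each time a character uses it.
; BeginPlay caches closed and open yaw rotations for the Sphere component.
; OnUsed fires an event whose FlipFlop plays or reverses a timeline, lerping Sphere's relative rotation between them.
; Focus functions toggle custom depth rendering on the static mesh.
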(event `self.ReceiveBeginPlay`
  (bind _relativerotation (`SceneComponent.RelativeRotation` (`self.Sphere`)))
  (set `self.Starting Rotation` _relativerotation)
  (set `self.End rotation` (`KismetMathLibrary.MakeRotator` (.roll _relativerotation) (.pitch _relativerotation) (- (.yaw _relativerotation) 86.0))))

(event `OnUsedd`
  (`/Engine/EditorBlueprintResources/StandardMacros.FlipFlop`
    (:`A`
      (bind (_direction _newtrack_0) (`Timeline|Timeline_0` :!label _label)
        (:`Update`
          (`SceneComponent.K2_SetRelativeRotation` (`self.Sphere`) (`KismetMathLibrary.RLerp` (`self.Starting Rotation`) (`self.End rotation`) _newtrack_0) false false))))
    (:`B`
      (goto _label :!via `Reverse`))))

(fn `EndFocusItem`
  (returns (ReturnValue :type Boolean))
  (`PrimitiveComponent.SetRenderCustomDepth` (`self.StaticMesh`) false)
  (return false))

(fn `OnUsed`
  (params (character :type "Character Object Reference"))
  (returns (ReturnValue :type Boolean))
  (`self.OnUsedd`)
  (return true))

(fn `StartFocusItem`
  (returns (ReturnValue :type Boolean))
  (`PrimitiveComponent.SetRenderCustomDepth` (`self.StaticMesh`) true)
  (return false))

(fn `UserConstructionScript`)