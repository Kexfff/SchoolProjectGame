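; Grass spawn area actor that shows an editable volume as a translucent procedural mesh, built in its construction script.
; A floor section with collision is built from the vertex and triangle arrays, then the vertices are copied upward by AreaHeight to form a ceiling section.
; Thin instanced pillars, scaled vertically by AreaHeight and placed at each floor vertex, visualize the area's height.
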(fn `UserConstructionScript`
  (bind _proceduralmesh (`self.ProceduralMesh`))
  (bind _proceduralmesh_2 (`self.ProceduralMesh`))
  (`ProceduralMeshComponent.CreateMeshSection_LinearColor` :`self` _proceduralmesh_2 :`Vertices` (`self.V`) :`Triangles` (`self.triangles`) :`bCreateCollision` true)
  (`PrimitiveComponent.SetMaterial` _proceduralmesh_2 0 "/Game/World/DynamicGrassLite/Materials/Misc/SimpleTranslucent_M.SimpleTranslucent_M")
  (`InstancedStaticMeshComponent.ClearInstances` (`self.HeightVisPillars`))
  (`KismetArrayLibrary.Array_Clear` (`self.V_Ceiling`))
  (for _array_element (`self.V`)
    (`KismetArrayLibrary.Array_Add` (`self.V_Ceiling`) (+ _array_element (`KismetMathLibrary.MakeVector` 0.0 0.0 (`self.areaHeight`))))
    (`InstancedStaticMeshComponent.AddInstance` (`self.HeightVisPillars`) (`KismetMathLibrary.MakeTransform` _array_element (struct) (`KismetMathLibrary.MakeVector` 0.01 0.01 (`self.areaHeight`)))))
  (`ProceduralMeshComponent.CreateMeshSection_LinearColor` :`self` _proceduralmesh :`SectionIndex` 1 :`Vertices` (`self.V_Ceiling`) :`Triangles` (`self.triangles`))
  (`PrimitiveComponent.SetMaterial` _proceduralmesh 1 "/Game/World/DynamicGrassLite/Materials/Misc/SimpleTranslucent_M.SimpleTranslucent_M"))