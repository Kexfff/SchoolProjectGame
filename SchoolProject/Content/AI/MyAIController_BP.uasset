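; AI controller that sends its controlled character toward the player when perception updates.
; Either of two AIPerception components triggers the same logic: a living pawn moves to within a set radius of player pawn 0, and an MyFPCharacter_BP pawn gets its IsSighting flag set.
; The perceived actors are ignored.
; Behavior tree startup and Blackboard "Enemy" assignment are present but disconnected.
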(event `self.ReceiveBeginPlay`)

(event `self.AIPerception.OnPerceptionUpdated`
  (params (UpdatedActors :type "Array of Actor Object Reference (by ref)"))
  (bind _asbasic_character_class (cast `/Game/Actor/BasicCharacterClass` (`self.K2_GetPawn`) :!label _label))
  (if (not (`/Game/Actor/BasicCharacterClass.IsDead` _asbasic_character_class))
    (`self.MoveToActor` (`GameplayStatics.GetPlayerPawn` 0) 1000.0 true true true null)
    (bind _asmy_fpcharacter_bp (cast `/Game/Actor/Player/MyFPCharacter_BP` _asbasic_character_class))
    (set `/Game/Actor/Player/MyFPCharacter_BP.IsSighting` true _asmy_fpcharacter_bp)))

(event `self.AIPerception1.OnPerceptionUpdated`
  (params (UpdatedActors :type "Array of Actor Object Reference (by ref)"))
  (goto _label))

(fn `UserConstructionScript`)