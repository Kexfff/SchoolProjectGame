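; AI controller for prey that runs Prey_BahaviourTree and feeds it flee data from AI perception.
; Perception updates for MyFPCharacter_BP copy the sensed state to IsGoalFound; other actors clear it.
; Player updates, sensed or lost, also seek a random reachable point around an origin projected away from the player for Location.
; Random pure nodes re-evaluate, so the stored point differs from the one checked.
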(event `self.ReceiveBeginPlay`
  (`self.RunBehaviorTree` "/Game/Actor/Animals/Prey_BahaviourTree.Prey_BahaviourTree"))

(event `self.AIPerception.OnTargetPerceptionUpdated`
  (params (Actor :type "Actor Object Reference") (Stimulus :type "AIStimulus Structure"))
  (bind _returnvalue (`AIBlueprintHelperLibrary.GetBlackboard` null))
  (bind _returnvalue_2 (`KismetMathLibrary.RandomFloatInRange` -1000.0 -5000.0))
  (bind _returnvalue_3 (`self.K2_GetActorLocation` (`self.K2_GetPawn`)))
  (bind (_randomlocation _returnvalue_4) (`NavigationSystemV1.K2_GetRandomReachablePointInRadius` (+ _returnvalue_3 (* (`KismetMathLibrary.GetForwardVector` (`KismetMathLibrary.FindLookAtRotation` _returnvalue_3 (`self.K2_GetActorLocation` Actor))) _returnvalue_2)) (+ (`KismetMathLibrary.Abs` _returnvalue_2) (`KismetMathLibrary.RandomFloatInRange` 200.0 2000.0)) null null))
  (cast `/Game/Actor/Player/MyFPCharacter_BP` Actor
    (:`then`
      (`BlackboardComponent.SetValueAsBool` _returnvalue "IsGoalFound" (`.bSuccessfullySensed` (break `AIStimulus` Stimulus)))
      (if _returnvalue_4
        (`BlackboardComponent.SetValueAsVector` _returnvalue "Location" _randomlocation)))
    (:`CastFailed`
      (`BlackboardComponent.SetValueAsBool` _returnvalue "IsGoalFound" false))))

(fn `UserConstructionScript`)