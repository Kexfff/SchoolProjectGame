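; BasicTest is a pickup item actor that adds itself to the player's inventory when used.
; On BeginPlay it rebuilds its inventory struct with a reference to itself, keeping the other fields.
; Focus functions toggle custom depth rendering on its static mesh.
; OnUsed casts the user to MyFPCharacter_BP, passes InventoryClass to AddItem, then destroys the actor.
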(event `self.ReceiveBeginPlay`
  (bind (_item _itemimage _pickuptext _actiontext _itemref _isusable) (break `/Game/Blueprints/Inventory/InventoryStruct` (`self.InvStruct`)))
  (set `self.InvStruct` (make `/Game/Blueprints/Inventory/InventoryStruct` null _itemimage _pickuptext _actiontext self _isusable)))

(fn `EndFocusItem`
  (returns (ReturnValue :type Boolean))
  (`PrimitiveComponent.SetRenderCustomDepth` (`self.StaticMesh`) false)
  (return true))

(fn `OnUsed`
  (params (character :type "Character Object Reference"))
  (returns (ReturnValue :type Boolean))
  (bind _asmy_fpcharacter_bp (cast `/Game/Actor/MyFPCharacter_BP` character))
  (`/Game/Actor/MyFPCharacter_BP.AddItem` _asmy_fpcharacter_bp (`self.InventoryClass`))
  (`self.K2_DestroyActor`)
  (return true))

(fn `StartFocusItem`
  (returns (ReturnValue :type Boolean))
  (`PrimitiveComponent.SetRenderCustomDepth` (`self.StaticMesh`) true)
  (return false))

(fn `UserConstructionScript`)