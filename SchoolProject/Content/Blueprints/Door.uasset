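; Door actor that can be focused and used, with placeholder use behavior that only prints "Hello".
; Focus start and end toggle custom depth rendering on its static mesh, the usual hook for an outline highlight.
; On spawn it sets the mesh's relative scale from the passed options, while its ComponentsToSave function returns nothing and the event graph is empty.
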(event `self.ReceiveBeginPlay`)

(fn `ComponentsToSave`
  (returns (Components :type "Array of ActorComponent Object Reference") (Components :type "Array of ActorComponent Object Reference"))
  (return))

(fn `EndFocusItem`
  (returns (ReturnValue :type Boolean))
  (`PrimitiveComponent.SetRenderCustomDepth` (`self.StaticMesh`) false)
  (return true))

(fn `OnSpawned`
  (params (Options :type "/Game/Blueprints/Inventory/InventoryStruct Structure"))
  (`SceneComponent.SetRelativeScale3D` (`self.StaticMesh`) (`KismetMathLibrary.Conv_DoubleToVector` (`.Scale_33_7C13E0F34BFC0FEFFBA216A482E11CB0` (break `/Game/Blueprints/Inventory/InventoryStruct` Options)))))

(fn `OnUsed`
  (params (character :type "Character Object Reference"))
  (returns (ReturnValue :type Boolean))
  (`KismetSystemLibrary.PrintString` "Hello"))

(fn `StartFocusItem`
  (returns (ReturnValue :type Boolean))
  (`PrimitiveComponent.SetRenderCustomDepth` (`self.StaticMesh`) true)
  (return false))

(fn `UserConstructionScript`)