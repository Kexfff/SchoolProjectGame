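; Pickup actor that shows a prompt widget while the player is inside its trigger and can be collected into the HUD inventory.
; The construction script applies the custom mesh and fills the item struct, and BeginPlay binds to the character's PickupItem dispatcher.
; Collecting adds the struct, refreshes the inventory and hides the actor without destroying it.
; UseAction spawns a fire effect at the character's drop location, then destroys the actor.
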(event `self.ReceiveBeginPlay`
  (bind _iteminfo (`self.ItemInfo`))
  (bind (_item _itemimage _pickuptext) (break `/Game/Blueprints/InventoryStruct` _iteminfo))
  ;[1 1 1] Event begin play
  (bind _returnvalue (`|CreateWidget` "/Game/Actor/HUD/UMG/PickupText.PickupText_C"))
  (set `self.PickupTextWidget` _returnvalue)
  (set `/Game/Actor/HUD/UMG/PickupText.PickupActor` _item _returnvalue)
  (set `/Game/Actor/HUD/UMG/PickupText.PickupText` _pickuptext _returnvalue)
  (setmembers `/Game/Blueprints/InventoryStruct` :`StructRef` _iteminfo :`Item` self)
  (bind _asmy_fpcharacter_bp (cast `/Game/Actor/MyFPCharacter_BP` (`GameplayStatics.GetPlayerCharacter` 0)))
  (bind _output_get (set `self.MyCharacter` _asmy_fpcharacter_bp))
  (add `/Game/Actor/MyFPCharacter_BP.PickupItem` _output_get (delegate `PickupItem_Event_0`)))

(event `PickupItem_Event_0`
  (bind _gamehudwidget (`/Game/Actor/MyFPCharacter_BP.GameHUDWidget` (`self.MyCharacter`)))
  ;[1 1 1] pickup item to inv
  (if (and (`self.GetActorEnableCollision`) (`self.IsInRange`))
    (`KismetArrayLibrary.Array_Add` (`/Game/Actor/HUD/UMG/GameHUD.Inventory_arr` _gamehudwidget) (`self.ItemInfo`))
    (`Widget.RemoveFromParent` (`self.PickupTextWidget`))
    (`self.SetActorHiddenInGame` true)
    (`self.SetActorEnableCollision` false)
    (`/Game/Actor/HUD/UMG/GameHUD.RefreshInventory` _gamehudwidget)))

(event `self.Trigger1.OnComponentBeginOverlap`
  (params (OverlappedComponent :type "PrimitiveComponent Object Reference") (OtherActor :type "Actor Object Reference") (OtherComp :type "PrimitiveComponent Object Reference") (OtherBodyIndex :type Integer) (bFromSweep :type Boolean) (SweepResult :type "HitResult Structure (by ref)"))
  ;[1 1 1] Triggers
  (cast `/Game/Actor/MyFPCharacter_BP` OtherActor)
  (`UserWidget.AddToViewport` (`self.PickupTextWidget`) 0)
  (set `self.IsInRange` true))

(event `self.Trigger1.OnComponentEndOverlap`
  (params (OverlappedComponent :type "PrimitiveComponent Object Reference") (OtherActor :type "Actor Object Reference") (OtherComp :type "PrimitiveComponent Object Reference") (OtherBodyIndex :type Integer))
  ;[1 1 1] Triggers
  (cast `/Game/Actor/MyFPCharacter_BP` OtherActor)
  (`Widget.RemoveFromParent` (`self.PickupTextWidget`))
  (set `self.IsInRange` false))

(event `/Game/Actor/HUD/ActionInteface.UseAction`
  ;[1 1 1] Add new features here!!!
  (`|SpawnActorFromClass` "/Game/StarterContent/Blueprints/Blueprint_Effect_Fire.Blueprint_Effect_Fire_C" (`SceneComponent.K2_GetComponentToWorld` (`/Game/Actor/MyFPCharacter_BP.DropLocation` (`self.MyCharacter`))) "Undefined" "OverrideRootScale" null null)
  (`self.K2_DestroyActor`))

(fn `UserConstructionScript`
  (setmembers `/Game/Blueprints/InventoryStruct` :`StructRef` (`self.ItemInfo`) :`Item` self :`ItemImage` (`self.InventoryImage`) :`PickupText` (`self.PickupText`) :`ActionText` (`self.ActionText`))
  (`StaticMeshComponent.SetStaticMesh` (`self.Can`) (`self.CustomMesh`)))