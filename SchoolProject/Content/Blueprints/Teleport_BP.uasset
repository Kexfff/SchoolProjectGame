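; Teleport_BP is an interactable object that loads another level when a character uses it.
; OnUsed fires the OnUsedd event, which opens the level named in LevelName unless it is None, then reports the use as handled.
; Focus start and end toggle custom depth rendering on its static mesh, likely driving a highlight outline.
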(event `self.ReceiveBeginPlay`)

(event `OnUsedd`
  (bind _levelname (`self.LevelName`))
  (if (!= _levelname "None")
    (`GameplayStatics.OpenLevel` _levelname)))

(fn `EndFocusItem`
  (returns (ReturnValue :type Boolean))
  (`PrimitiveComponent.SetRenderCustomDepth` (`self.StaticMesh`) false)
  (return false))

(fn `OnUsed`
  (params (character :type "Character Object Reference"))
  (returns (ReturnValue :type Boolean))
  (`self.OnUsedd`)
  (return true))

(fn `StartFocusItem`
  (returns (ReturnValue :type Boolean))
  (`PrimitiveComponent.SetRenderCustomDepth` (`self.StaticMesh`) true)
  (return false))

(fn `UserConstructionScript`)